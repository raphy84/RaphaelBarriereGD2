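; BPC_ColecteCour is a component that handles collecting objects for score.
; On BeginPlay it casts and caches the BP_GameInstance.
; Collect adds the passed object's ValueScore to the Score held in that game instance, then destroys the object's owning actor through the Destroy event.
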(event Custom|Destroy
  (params (Target :type Actor%20Object%20Reference))
  (Actor|DestroyActor Target))

(event EventBeginPlay
  (bind _asbp_game_instance (Utilities|Casting|CastToBP_GameInstance (Game|GetGameInstance)))
  (Variables|Default|SetAs%20BP%20Game%20Instance _asbp_game_instance))

(event EventTick
  (params (DeltaSeconds :type Float%20%28single-precision%29)))

(fn Collect
  (params (CollectObjet :type BPC%20Colecte%20Cour%20Object%20Reference))
  (Variables|/Game/GameCour/BP_GameInstance.BP_GameInstance_C|SetScore (Variables|Default|GetAs%20BP%20Game%20Instance) (+ (Variables|/Game/GameCour/BP_GameInstance.BP_GameInstance_C|GetScore (Variables|Default|GetAs%20BP%20Game%20Instance)) (Variables|BPC_ColecteCour_C|GetValueScore CollectObjet)))
  (CallFunction|Destroy (Components|GetOwner CollectObjet)))